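; Player state for the Prop Hunt gameplay mode, holding a player's randomized appearance and handling assignment to the Hunter role.
; On BeginPlay, the server randomly picks gender and color ID, then flags the appearance as initialized.
; The IsHunter RepNotify, acting only on authority, registers the player with the game state's Hunter team and has the game mode spawn a Hunter character at a Hunter start with that appearance.
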(event `self.ReceiveBeginPlay`
  (`self.Generate_Appearance`))

(fn `Generate_Appearance`
  (`/Engine/EditorBlueprintResources/ActorMacros.Switch Has Authority`
    (:`Authority`
      (set `self.Appearance_Male?` (`KismetMathLibrary.RandomBool`))
      (set `self.Appearance_ColorID` (`KismetMathLibrary.RandomIntegerInRange` 0 4))
      (set `self.Appearance_Initialized?` true))))

(fn `OnRep_IsHunter?`
  (`/Engine/EditorBlueprintResources/ActorMacros.Switch Has Authority`
    (:`Authority`
      ;[0.05098 0.05098 0.05098] Add ourselves to the Hunter Team
      (bind _asbp_gs_gameplay (cast `/Game/PropHunt/Blueprints/Core/Gameplay/Core/BP_GS_Gameplay` (`GameplayStatics.GetGameState`)))
      (`/Game/PropHunt/Blueprints/Core/Gameplay/Core/BP_GS_Gameplay.Add_Hunter` _asbp_gs_gameplay self)
      ;[0.05098 0.05098 0.05098] Spawn ourselves a Hunter Character
      (bind _asbp_gm_gameplay (cast `/Game/PropHunt/Blueprints/Core/Gameplay/Core/BP_GM_Gameplay` (`GameplayStatics.GetGameMode`)))
      (`/Game/PropHunt/Blueprints/Core/Gameplay/Core/BP_GM_Gameplay.Spawn_Character_Hunter` _asbp_gm_gameplay (`self.GetPlayerController`) "Hunter" (`self.Appearance_Male?`) (`self.Appearance_ColorID`)))))

(fn `UserConstructionScript`)